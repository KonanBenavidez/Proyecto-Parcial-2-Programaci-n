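; BP_Shooter is a mana-limited shooter that fires a projectile from its SpawnPoint on left mouse press.
; Each shot plays a sound, spends ManaPerShot, prints the remaining mana and waits FireRate.
; When mana runs out, a delay adds MaxMana and loops back to fire again without a new press.
; Pressing while empty calls StartRecharge, which only zeroes mana after RechargeTime.
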(event `StartRecharge`
  (if (<= (`self.CurrentMana`) 0.0)
    (`KismetSystemLibrary.Delay` (`self.RechargeTime`))
    (bind _output_get (set `self.CurrentMana` 0.0))))

(event `Key|LeftMouseButton`
  (params (Key :type "Key Structure"))
  (:`Pressed`
    (if (> (`self.CurrentMana`) 0.0) :!label _label
      (`|SpawnActorFromClass` (`self.ProjectileClass`) (`SceneComponent.K2_GetComponentToWorld` (`self.SpawnPoint`)) "AlwaysSpawn" "MultiplyWithRoot" null null)
      (`GameplayStatics.PlaySound2D` "/Game/StarterContent/Audio/Collapse_Cue.Collapse_Cue" 1.0 1.0 0.0 null null)
      (bind _output_get (set `self.CurrentMana` (- (`self.CurrentMana`) (`self.ManaPerShot`))))
      (`KismetSystemLibrary.PrintString` (`KismetStringLibrary.Conv_DoubleToString` _output_get))
      (`KismetSystemLibrary.Delay` (`self.FireRate`))
      (if (<= (`self.CurrentMana`) 0.0)
        (`KismetSystemLibrary.Delay` (`self.RechargeTime`))
        (set `self.CurrentMana` (+ (`self.CurrentMana`) (`self.MaxMana`)))
        (goto _label))
      (else
        (`self.StartRecharge`)
        (if true
          _)))))

(fn `UserConstructionScript`)